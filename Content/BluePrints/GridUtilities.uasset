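; Grid utility functions that convert between world positions and integer 3D grid coordinates.
; GetGridSize supplies a fixed cell size of 100 units to both conversions.
; WorldToGrid keeps the whole part of each axis divided by that size, truncating toward zero rather than flooring negative coordinates.
; GridToWorld multiplies back by the size with no half-cell centering offset.
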(fn `GetGridSize`
  (returns (`Grid Size` :type Integer))
  (return 100))

(fn `GridToWorld`
  (params (GridLocation :type "IntVector Structure"))
  (returns (Position :type "Vector Structure"))
  (bind _grid_size (`self.GetGridSize` null))
  (return (`KismetMathLibrary.MakeVector` (`KismetMathLibrary.Conv_IntToDouble` (* GridLocation_X _grid_size)) (`KismetMathLibrary.Conv_IntToDouble` (* GridLocation_Y _grid_size)) (`KismetMathLibrary.Conv_IntToDouble` (* GridLocation_Z _grid_size)))))

(fn `WorldToGrid`
  (params (Position :type "Vector Structure"))
  (returns (GridLocation :type "IntVector Structure"))
  (bind _grid_size (`self.GetGridSize` null))
  (return (make `IntVector` (`.ReturnValue` (`KismetMathLibrary.FMod` Position_X (`KismetMathLibrary.Conv_IntToDouble` _grid_size))) (`.ReturnValue` (`KismetMathLibrary.FMod` Position_Y (`KismetMathLibrary.Conv_IntToDouble` _grid_size))) (`.ReturnValue` (`KismetMathLibrary.FMod` Position_Z (`KismetMathLibrary.Conv_IntToDouble` _grid_size))))))
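; AI path Blueprint that serves looping, grid-aligned waypoints from a spline.
; GetNextSplinePoint reads the current point's world location, snaps it through WorldToGrid and GridToWorld with Z zeroed, and returns X and Y.
; It then advances the index, wrapping at the last point.
; CancelMovement steps the index back by one without wrapping, and the event graph is unused.
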(fn `CancelMovement`
  (`/Engine/EditorBlueprintResources/StandardMacros.DecrementInt` (`self.CurrentSplinePoint`)))

(fn `GetNextSplinePoint`
  (returns (SplinePoint :type "Vector2D Structure"))
  (locals (TempLocation :type "Vector Structure"))
  (bind _spline (`self.Spline`))
  (bind _output_get (set `local.TempLocation` (`SplineComponent.GetLocationAndTangentAtSplinePoint` _spline (`self.CurrentSplinePoint`) "World")))
  (bind _gridlocation (`/Game/BluePrints/GridUtilities.WorldToGrid` (`KismetMathLibrary.MakeVector` (.x _output_get) (.y _output_get))))
  (bind _position (`/Game/BluePrints/GridUtilities.GridToWorld` _gridlocation))
  (set `self.CurrentSplinePoint` (mod (+ (`self.CurrentSplinePoint`) 1) (`SplineComponent.GetNumberOfSplinePoints` _spline)))
  (return (`KismetMathLibrary.MakeVector2D` (.x _position) (.y _position))))

(fn `UserConstructionScript`)
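; Enemy AI that patrols a spline Path and damages the player while it can see them.
; Construction snaps it to the first spline point; at runtime it loops AIMoveTo between points with a pause.
; AIPerception detecting a GridCharacter halts patrol and enables damage over time on Tick, resuming patrol when sight is lost.
; AnyDamage lowers health, shown on an AIHealth widget bar; the overlap-enabled Attack input only prints.
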(event `self.ReceiveAnyDamage`
  (params (Damage :type "Float (single-precision)") (DamageType :type "DamageType Object Reference") (InstigatedBy :type "Controller Object Reference") (DamageCauser :type "Actor Object Reference"))
  (set `self.EniHealth` (- (`self.EniHealth`) Damage)))

(event `self.ReceiveBeginPlay`
  (`self.MoveToPoint`)
  (bind _asaihealth (cast `/Game/UI_Assets/Health/AIHealth` (`WidgetComponent.GetUserWidgetObject` (`self.Widget`))))
  (set `/Game/UI_Assets/Health/AIHealth.OwningAI` self _asaihealth))

(event `self.Box.OnComponentBeginOverlap`
  (params (OverlappedComponent :type "PrimitiveComponent Object Reference") (OtherActor :type "Actor Object Reference") (OtherComp :type "PrimitiveComponent Object Reference") (OtherBodyIndex :type Integer) (bFromSweep :type Boolean) (SweepResult :type "HitResult Structure (by ref)"))
  ;[1 1 1] Player Damages Enemy
  (`self.EnableInput` (`GameplayStatics.GetPlayerController` 0))
  (`KismetSystemLibrary.PrintString` "Entered Trigger"))

(event `self.Box.OnComponentEndOverlap`
  (params (OverlappedComponent :type "PrimitiveComponent Object Reference") (OtherActor :type "Actor Object Reference") (OtherComp :type "PrimitiveComponent Object Reference") (OtherBodyIndex :type Integer))
  ;[1 1 1] Player Damages Enemy
  (`self.DisableInput` (`GameplayStatics.GetPlayerController` 0)))

(event `MoveToPoint`
  (bind (_returnvalue_x _returnvalue_y _returnvalue_z) (`KismetMathLibrary.BreakVector` (`self.K2_GetActorLocation`)))
  (bind _path (`self.Path`))
  ;[1 1 1] Patrol Movement
  (if (`KismetSystemLibrary.IsValid` _path)
    (bind _splinepoint (`/Game/BluePrints/AI/AIPath.GetNextSplinePoint` _path))
    (`self.K2_SetActorRotation` (`KismetMathLibrary.FindLookAtRotation` (`self.K2_GetActorLocation`) (`KismetMathLibrary.MakeVector` (`KismetMathLibrary.BreakVector2D` _splinepoint) (`.Y` (`KismetMathLibrary.BreakVector2D` _splinepoint)) _returnvalue_z)))
    (`KismetSystemLibrary.DrawDebugPoint` (`KismetMathLibrary.MakeVector` (`KismetMathLibrary.BreakVector2D` _splinepoint) (`.Y` (`KismetMathLibrary.BreakVector2D` _splinepoint)) 100.0) 25.0 (struct :`G` 0.8604 :`B` 1.0 :`A` 1.0) 100.0)
    (bind _movementresult (`|AIMoveTo` self (`KismetMathLibrary.MakeVector` (`KismetMathLibrary.BreakVector2D` _splinepoint) (`.Y` (`KismetMathLibrary.BreakVector2D` _splinepoint)) _returnvalue_z) null 20.0)
      (:`OnSuccess`
        (`KismetSystemLibrary.Delay` 3.0)
        (`self.MoveToPoint`))
      (:`OnFail`
        (`KismetSystemLibrary.PrintString` (`|GetEnumeratorNameAsString` _movementresult))))))

(event `InputAction|Attack`
  (params (Key :type "Key Structure"))
  ;[1 1 1] Player Damages Enemy
  (:`Pressed`
    (`KismetSystemLibrary.PrintString` "Attacked Enemy")))

(event `self.ReceiveTick`
  (params (DeltaSeconds :type "Float (single-precision)"))
  (bind _widget (`self.Widget`))
  (bind _returnvalue (`SceneComponent.K2_GetComponentLocation` _widget))
  (if (`self.PlayerSeen`)
    (`GameplayStatics.ApplyDamage` (`self.PlayerTarget`) (* DeltaSeconds 10.0)))
  ;[1 1 1] Enemy Health Bar
  (bind _asaihealth (cast `/Game/UI_Assets/Health/AIHealth` (`WidgetComponent.GetUserWidgetObject` (`self.Widget`))))
  (`ProgressBar.SetPercent` (`/Game/UI_Assets/Health/AIHealth.ProgressBar_103` _asaihealth) (/ (`self.EniHealth`) 100.0))
  (`SceneComponent.K2_SetWorldRotation` _widget (`KismetMathLibrary.FindLookAtRotation` _returnvalue (+ _returnvalue (0.0 0.0 100.0))) false false))

(event `self.AIPerception.OnPerceptionUpdated`
  (params (UpdatedActors :type "Array of Actor Object Reference"))
  (bind _info (`AIPerceptionComponent.GetActorsPerception` (`self.AIPerception`) (`|GetArrayItem` UpdatedActors)))
  (bind _asgrid_character (cast `/Game/BluePrints/GridCharacter` (break `ActorPerceptionBlueprintInfo` _info)))
  (set `self.PlayerTarget` _asgrid_character)
  (bind (_output_age _output_expirationage _output_strength _output_stimuluslocation _output_receiverlocation _output_tag _output_bsuccessfullysensed) (break `AIStimulus` (`|GetArrayItem` (`.LastSensedStimuli` (break `ActorPerceptionBlueprintInfo` _info)))))
  (if _output_bsuccessfullysensed
    (set `self.PlayerSeen` true)
    (`KismetSystemLibrary.PrintString` "Player Detected")
    ;[1 1 1] cancel movement when seeing player
    (if (`self.PlayerSeen`)
      (`Controller.StopMovement` (`self.GetController`))
      (`/Game/BluePrints/AI/AIPath.CancelMovement` (`self.Path`)))
    (else
      (set `self.PlayerSeen` false)
      (`KismetSystemLibrary.PrintString` "Player Not Seen")
      (`self.MoveToPoint`))))

(fn `UserConstructionScript`
  (bind _path (`self.Path`))
  (bind (_location _tangent) (`SplineComponent.GetLocationAndTangentAtSplinePoint` (`/Game/BluePrints/AI/AIPath.Spline` _path) 0 "World"))
  (if (`KismetSystemLibrary.IsValid` _path)
    (`self.K2_SetActorLocation` _location)
    (`self.K2_SetActorLocationAndRotation` _location (`KismetMathLibrary.FindLookAtRotation` _location _tangent))))
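; Enemy actor for a grid-based game that snaps to its grid cell on BeginPlay and shows a health bar.
; Its trigger box toggles player input on overlap, so the Attack action reaches the enemy, though it currently only prints a message.
; Tick pushes EniHealth into the AIHealth widget's progress bar and rotates that widget to face straight up.
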(event `self.ReceiveBeginPlay`
  (bind _gridlocation (`/Game/BluePrints/GridUtilities.WorldToGrid` (`self.K2_GetActorLocation`)))
  (bind _output_get (set `self.CurrentGridLocation` _gridlocation))
  (bind _position (`/Game/BluePrints/GridUtilities.GridToWorld` _output_get))
  (`self.K2_SetActorLocation` _position false true))

(event `self.Box.OnComponentBeginOverlap`
  (params (OverlappedComponent :type "PrimitiveComponent Object Reference") (OtherActor :type "Actor Object Reference") (OtherComp :type "PrimitiveComponent Object Reference") (OtherBodyIndex :type Integer) (bFromSweep :type Boolean) (SweepResult :type "HitResult Structure (by ref)"))
  ;[1 1 1] Player Damages Enemy
  (`self.EnableInput` (`GameplayStatics.GetPlayerController` 0))
  (`KismetSystemLibrary.PrintString` "Entered Trigger"))

(event `self.Box.OnComponentEndOverlap`
  (params (OverlappedComponent :type "PrimitiveComponent Object Reference") (OtherActor :type "Actor Object Reference") (OtherComp :type "PrimitiveComponent Object Reference") (OtherBodyIndex :type Integer))
  ;[1 1 1] Player Damages Enemy
  (`self.DisableInput` (`GameplayStatics.GetPlayerController` 0)))

(event `InputAction|Attack`
  (params (Key :type "Key Structure"))
  ;[1 1 1] Player Damages Enemy
  (:`Pressed`
    (`KismetSystemLibrary.PrintString` "Attacked Enemy")))

(event `self.ReceiveTick`
  (params (DeltaSeconds :type "Float (single-precision)"))
  (bind _widget (`self.Widget`))
  (bind _returnvalue (`SceneComponent.K2_GetComponentLocation` _widget))
  ;[1 1 1] Enemy Health Bar
  (bind _asaihealth (cast `/Game/UI_Assets/Health/AIHealth` (`WidgetComponent.GetUserWidgetObject` (`self.Widget`))))
  (`ProgressBar.SetPercent` (`/Game/UI_Assets/Health/AIHealth.ProgressBar_103` _asaihealth) (/ (`self.EniHealth`) 100.0))
  (`SceneComponent.K2_SetWorldRotation` _widget (`KismetMathLibrary.FindLookAtRotation` _returnvalue (+ _returnvalue (0.0 0.0 100.0))) false false))

(fn `UserConstructionScript`)
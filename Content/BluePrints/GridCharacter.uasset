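; Player character for grid-based movement as a parasite that snaps to the grid on BeginPlay and steps one cell per directional input.
; Each step rotates the actor, sphere-traces forward for blockers, then lerps to the cell via a timeline and updates the grid location.
; Enter toggles between parasite and scientist host forms; only the parasite briefly swaps mesh when moving.
; A custom event removes a random level name and opens another at random.
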(event `self.ReceiveBeginPlay`
  (bind _gridlocation (`/Game/BluePrints/GridUtilities.WorldToGrid` (`self.K2_GetActorLocation`)))
  (bind _output_get (set `self.CurrentGridLocation` _gridlocation))
  (bind _position (`/Game/BluePrints/GridUtilities.GridToWorld` _output_get))
  (`self.K2_SetActorLocation` _position false true))

(event `CustomEvent_0`
  (bind _levelnames (`self.LevelNames`))
  (bind _returnvalue (`KismetMathLibrary.RandomIntegerInRange` 0 (`KismetArrayLibrary.Array_Length` (`self.LevelNames`))))
  (`KismetArrayLibrary.Array_Remove` _levelnames _returnvalue)
  (`GameplayStatics.OpenLevel` (`|GetArrayItem` _levelnames _returnvalue)))

(event `Key|Enter`
  (params (Key :type "Key Structure"))
  (:`Pressed`
    (`/Engine/EditorBlueprintResources/StandardMacros.FlipFlop`
      (:`A`
        (`StaticMeshComponent.SetStaticMesh` (`self.Parasite`) "/Game/BluePrints/scientistv2.scientistv2")
        (`self.SetActorScale3D` (1.5 1.5 1.5))
        (set `self.Host` true))
      (:`B`
        (`StaticMeshComponent.SetStaticMesh` (`self.Parasite`) "/Game/Characters/Para_ani_1/Parasite1.Parasite1")
        (`self.SetActorScale3D` (1.0 1.0 1.0))
        (set `self.Host` false)))))

(event `InputAction|Move Backward`
  (params (Key :type "Key Structure"))
  (bind (_returnvalue_x _returnvalue_y _returnvalue_z) (`KismetMathLibrary.BreakVector` (`self.K2_GetActorLocation`)))
  (bind (_currentgridlocation_x _currentgridlocation_y _currentgridlocation_z) (break `IntVector` (`self.CurrentGridLocation`)))
  ;[1 1 1] Move Down
  (:`Pressed`
    (if (not (`self.bMoving`))
      (bind _position (`/Game/BluePrints/GridUtilities.GridToWorld` (make `IntVector` (- _currentgridlocation_x 1) _currentgridlocation_y _currentgridlocation_z)))
      (`self.K2_SetActorRotation` (`KismetMathLibrary.RotatorFromAxisAndAngle` (0.0 0.0 90.0) 180.0))
      (`self.MoveToWithoutNavigation` (`KismetMathLibrary.MakeVector` (.x _position) (.y _position) _returnvalue_z) 1.0)
      (if (not (`self.Host`))
        (`StaticMeshComponent.SetStaticMesh` (`self.Parasite`) "/Game/Characters/Para_ani_2/Parasite2.Parasite2")
        (`KismetSystemLibrary.Delay` 0.2)
        (`StaticMeshComponent.SetStaticMesh` (`self.Parasite`) "/Game/Characters/Para_ani_1/Parasite1.Parasite1")
        (`KismetSystemLibrary.PrintText` (`|FormatText` "Back = {0} {1} {2}" (.x _position) (.y _position) _returnvalue_z))))))

(event `InputAction|Move Forward`
  (params (Key :type "Key Structure"))
  (bind (_returnvalue_x _returnvalue_y _returnvalue_z) (`KismetMathLibrary.BreakVector` (`self.K2_GetActorLocation`)))
  (bind (_currentgridlocation_x _currentgridlocation_y _currentgridlocation_z) (break `IntVector` (`self.CurrentGridLocation`)))
  ;[1 1 1] Move Up
  (:`Pressed`
    (if (not (`self.bMoving`))
      (bind _position (`/Game/BluePrints/GridUtilities.GridToWorld` (make `IntVector` (+ _currentgridlocation_x 1) _currentgridlocation_y _currentgridlocation_z)))
      (`self.K2_SetActorRotation` (`KismetMathLibrary.RotatorFromAxisAndAngle` (0.0 0.0 90.0)))
      (`self.MoveToWithoutNavigation` (`KismetMathLibrary.MakeVector` (.x _position) (.y _position) _returnvalue_z) 1.0)
      (if (not (`self.Host`))
        (`StaticMeshComponent.SetStaticMesh` (`self.Parasite`) "/Game/Characters/Para_ani_2/Parasite2.Parasite2")
        (`KismetSystemLibrary.Delay` 0.2)
        (`StaticMeshComponent.SetStaticMesh` (`self.Parasite`) "/Game/Characters/Para_ani_1/Parasite1.Parasite1")
        (`KismetSystemLibrary.PrintText` (`|FormatText` "Forward = {0} {1} {2}" (.x _position) (.y _position) _returnvalue_z))))))

(event `MoveToWithoutNavigation`
  (params (TargetLocation :type "Vector Structure") (WalkDuration :type "Float (double-precision)"))
  ;[1 1 1] Player Collision Detector
  (bind _output_get (set `self.TempMoveActorLocation` (`self.K2_GetActorLocation`)))
  (bind _returnvalue (+ _output_get (0.0 0.0 0.0)))
  (bind (_outhit _returnvalue_2) (`KismetSystemLibrary.SphereTraceSingleForObjects` _returnvalue (+ _returnvalue (* (`self.GetActorForwardVector`) 100.0)) 15.0 (`|MakeArray` "ObjectTypeQuery1" "ObjectTypeQuery2" :!type "EObjectTypeQuery Enum") false (`|MakeArray` self :!type "Actor Object Reference")))
  (`KismetSystemLibrary.PrintString` (`KismetSystemLibrary.GetDisplayName` (`.HitActor` (`GameplayStatics.BreakHitResult` _outhit))))
  (if (not _returnvalue_2)
    (set `self.bMoving` true)
    (`TimelineComponent.SetPlayRate` (`self.Timeline_0`) (/ 3.0 WalkDuration))
    (bind (_direction _newtrack_0) (`Timeline|Timeline_0` :!via `PlayFromStart`)
      (:`Update`
        (`self.K2_SetActorLocation` (`KismetMathLibrary.VLerp` (`self.TempMoveActorLocation`) TargetLocation _newtrack_0)))
      (:`Finished`
        ;;[1 1 1] set current grid location after this node
        (set `self.bMoving` false)
        (bind _gridlocation (`/Game/BluePrints/GridUtilities.WorldToGrid` TargetLocation))
        (set `self.CurrentGridLocation` _gridlocation)))))

(event `InputAction|Move Right`
  (params (Key :type "Key Structure"))
  (bind (_returnvalue_x _returnvalue_y _returnvalue_z) (`KismetMathLibrary.BreakVector` (`self.K2_GetActorLocation`)))
  (bind (_currentgridlocation_x _currentgridlocation_y _currentgridlocation_z) (break `IntVector` (`self.CurrentGridLocation`)))
  ;[1 1 1] Move Right
  (:`Pressed`
    (if (not (`self.bMoving`))
      (bind _position (`/Game/BluePrints/GridUtilities.GridToWorld` (make `IntVector` _currentgridlocation_x (+ _currentgridlocation_y 1) _currentgridlocation_z)))
      (`self.K2_SetActorRotation` (`KismetMathLibrary.RotatorFromAxisAndAngle` (0.0 0.0 90.0) 90.0))
      (`self.MoveToWithoutNavigation` (`KismetMathLibrary.MakeVector` (.x _position) (.y _position) _returnvalue_z) 1.0)
      (if (not (`self.Host`))
        (`StaticMeshComponent.SetStaticMesh` (`self.Parasite`) "/Game/Characters/Para_ani_2/Parasite2.Parasite2")
        (`KismetSystemLibrary.Delay` 0.2)
        (`StaticMeshComponent.SetStaticMesh` (`self.Parasite`) "/Game/Characters/Para_ani_1/Parasite1.Parasite1")
        (`KismetSystemLibrary.PrintText` (`|FormatText` "Right = {0} {1} {2}" (.x _position) (.y _position) _returnvalue_z))))))

(event `InputAction|Move Left`
  (params (Key :type "Key Structure"))
  (bind (_returnvalue_x _returnvalue_y _returnvalue_z) (`KismetMathLibrary.BreakVector` (`self.K2_GetActorLocation`)))
  (bind (_currentgridlocation_x _currentgridlocation_y _currentgridlocation_z) (break `IntVector` (`self.CurrentGridLocation`)))
  ;[1 1 1] Move Left
  (:`Pressed`
    (if (not (`self.bMoving`))
      (bind _position (`/Game/BluePrints/GridUtilities.GridToWorld` (make `IntVector` _currentgridlocation_x (- _currentgridlocation_y 1) _currentgridlocation_z)))
      (`self.K2_SetActorRotation` (`KismetMathLibrary.RotatorFromAxisAndAngle` (0.0 0.0 90.0) 270.0))
      (`self.MoveToWithoutNavigation` (`KismetMathLibrary.MakeVector` (.x _position) (.y _position) _returnvalue_z) 1.0)
      (if (not (`self.Host`))
        (`StaticMeshComponent.SetStaticMesh` (`self.Parasite`) "/Game/Characters/Para_ani_2/Parasite2.Parasite2")
        (`KismetSystemLibrary.Delay` 0.2)
        (`StaticMeshComponent.SetStaticMesh` (`self.Parasite`) "/Game/Characters/Para_ani_1/Parasite1.Parasite1")
        (`KismetSystemLibrary.PrintText` (`|FormatText` "Left = {0} {1} {2}" (.x _position) (.y _position) _returnvalue_z))))))

(fn `UserConstructionScript`)
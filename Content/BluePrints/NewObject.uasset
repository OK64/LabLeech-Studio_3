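; Actor Blueprint that enables input on BeginPlay and moves itself from the Forward and Right axis inputs.
; Each axis event teleports the actor along world X or Y by a fixed step scaled by the axis value, without sweep or delta time.
; It then snaps to a fixed rotation chosen by the value's sign, with zero counting as negative.
; Overlap, Tick and construction are empty, and a SpawnActor node is unconnected.
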(event `self.ReceiveBeginPlay`
  (`self.EnableInput` null))

(event `self.ReceiveActorBeginOverlap`
  (params (OtherActor :type "Actor Object Reference")))

(event `InputAxis|Forward`
  (params (AxisValue :type "Float (single-precision)"))
  (`self.K2_SetActorTransform` (`KismetMathLibrary.Conv_VectorToTransform` (+ (`self.K2_GetActorLocation`) (* (100.0 0.0 0.0) AxisValue))) false true)
  (if (> AxisValue 0.0)
    (`self.K2_SetActorRotation` (struct))
    (else
      (`self.K2_SetActorRotation` (struct :`Yaw` 180.0)))))

(event `self.ReceiveTick`
  (params (DeltaSeconds :type "Float (single-precision)")))

(event `InputAxis|Right`
  (params (AxisValue :type "Float (single-precision)"))
  (`self.K2_SetActorTransform` (`KismetMathLibrary.Conv_VectorToTransform` (+ (`self.K2_GetActorLocation`) (* (0.0 100.0 0.0) AxisValue))) false true)
  (if (> AxisValue 0.0)
    (`self.K2_SetActorRotation` (struct :`Yaw` 90.0))
    (else
      (`self.K2_SetActorRotation` (struct :`Yaw` -90.0)))))

(fn `UserConstructionScript`)